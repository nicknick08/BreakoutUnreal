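; BP_MyBall is a bouncing ball actor that moves in the XZ plane and speeds up with every collision.
; BeginPlay picks a random X/Z direction, and Tick moves the ball by Velocity times Speed with a swept SetActorLocation.
; On Hit, a BP_MyBar deflects it along the vector from bar center to ball, while other surfaces mirror it about the hit normal.
; Each hit adds to Speed and prints it.
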(event EventBeginPlay
  ;[1 1 1] random verlocity
  (Variables|Default|SetVelocity (Math|Vector|MakeVector (Math|Random|RandomFloatinRange -1.0 1.0) 0.0 (Math|Random|RandomFloatinRange -1.0 1.0))))

(event Collision|EventActorBeginOverlap
  (params (OtherActor :type Actor%20Object%20Reference)))

(event EventTick
  (params (DeltaSeconds :type Float%20%28single-precision%29))
  ;[1 1 1] first move
  (Transformation|SetActorLocation (+ (Transformation|GetActorLocation) (* DeltaSeconds (* (Variables|Default|GetVelocity) (Variables|Default|GetSpeed)))) true false))

(event Collision|EventHit
  (params (MyComp :type Primitive%20Component%20Object%20Reference) (Other :type Actor%20Object%20Reference) (OtherComp :type Primitive%20Component%20Object%20Reference) (bSelfMoved :type Boolean) (HitLocation :type Vector :default "0, 0, 0") (HitNormal :type Vector :default "0, 0, 0") (NormalImpulse :type Vector :default "0, 0, 0") (Hit :type Hit%20Result%20Structure%20%28by%20ref%29))
  ;[1 1 1] when the ball hit the wall
  (bind _asbp_my_bar (Utilities|Casting|CastToBP_MyBar Other)
    (:then
      (Variables|Default|SetVelocity (Math|Vector|Normalize (- (Transformation|GetActorLocation) (Transformation|GetActorLocation _asbp_my_bar)))))
    (:CastFailed
      (Variables|Default|SetVelocity (Math|Vector|MakeVector (.X (Math|Vector|BreakVector (Math|Vector|MirrorVectorbyNormal (Variables|Default|GetVelocity) HitNormal))) 0.0 (.Z (Math|Vector|BreakVector (Math|Vector|MirrorVectorbyNormal (Variables|Default|GetVelocity) HitNormal)))))))
  (Variables|Default|SetSpeed (+ (Variables|Default|GetSpeed) 200))
  (Development|PrintString (Utilities|String|ToString(Integer) (Variables|Default|GetSpeed))))

(fn ConstructionScript)